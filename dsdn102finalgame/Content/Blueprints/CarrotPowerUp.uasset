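; Carrot pickup that temporarily grants the TopDownCharacter a triple jump when overlapped.
; On BeginPlay it binds actor overlap; a visible carrot raises JumpMaxCount, hides itself, then after a ten-second delay restores a double jump and reappears.
; The hidden state doubles as the cooldown guard, so the actor respawns without being destroyed.
; Component hit events are empty, and JumpPowerUp, a destroy-on-pickup variant, is not called here, while Respawn is empty.
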(event `self.ReceiveBeginPlay`
  (add `self.OnActorBeginOverlap` (delegate `OnActorBeginOverlap_Event`)))

(event `OnActorBeginOverlap_Event` :!signature `self.OnActorBeginOverlap`
  (params (OverlappedActor :type "Actor Object Reference") (OtherActor :type "Actor Object Reference"))
  (if (not (`self.bHidden`))
    (`KismetSystemLibrary.PrintString` "Visible")
    (bind _astop_down_character (cast `/Game/Blueprints/TopDownCharacter` OtherActor))
    (set `Character.JumpMaxCount` 3 _astop_down_character)
    (`self.SetActorHiddenInGame` true)
    (`KismetSystemLibrary.Delay` 10.0)
    (set `Character.JumpMaxCount` 2 _astop_down_character)
    (`self.SetActorHiddenInGame` false)))

(event `self.Cylinder.OnComponentHit`
  (params (HitComponent :type "PrimitiveComponent Object Reference") (OtherActor :type "Actor Object Reference") (OtherComp :type "PrimitiveComponent Object Reference") (NormalImpulse :type "Vector Structure") (Hit :type "HitResult Structure (by ref)")))

(event `self.Cone.OnComponentHit`
  (params (HitComponent :type "PrimitiveComponent Object Reference") (OtherActor :type "Actor Object Reference") (OtherComp :type "PrimitiveComponent Object Reference") (NormalImpulse :type "Vector Structure") (Hit :type "HitResult Structure (by ref)")))

(event `self.Sphere.OnComponentHit`
  (params (HitComponent :type "PrimitiveComponent Object Reference") (OtherActor :type "Actor Object Reference") (OtherComp :type "PrimitiveComponent Object Reference") (NormalImpulse :type "Vector Structure") (Hit :type "HitResult Structure (by ref)")))

(event `self.Sphere1.OnComponentHit`
  (params (HitComponent :type "PrimitiveComponent Object Reference") (OtherActor :type "Actor Object Reference") (OtherComp :type "PrimitiveComponent Object Reference") (NormalImpulse :type "Vector Structure") (Hit :type "HitResult Structure (by ref)")))

(event `self.Sphere2.OnComponentHit`
  (params (HitComponent :type "PrimitiveComponent Object Reference") (OtherActor :type "Actor Object Reference") (OtherComp :type "PrimitiveComponent Object Reference") (NormalImpulse :type "Vector Structure") (Hit :type "HitResult Structure (by ref)")))

(event `self.Sphere3.OnComponentHit`
  (params (HitComponent :type "PrimitiveComponent Object Reference") (OtherActor :type "Actor Object Reference") (OtherComp :type "PrimitiveComponent Object Reference") (NormalImpulse :type "Vector Structure") (Hit :type "HitResult Structure (by ref)")))

(fn `JumpPowerUp`
  (locals (NewLocalVar :type "SubmixEffectDelaySettings Structure"))
  (bind _astop_down_character (cast `/Game/Blueprints/TopDownCharacter` (`GameplayStatics.GetPlayerPawn` 0)))
  (set `Character.JumpMaxCount` 3 _astop_down_character)
  (`KismetSystemLibrary.PrintString` "jump count up")
  (`self.K2_DestroyActor`))

(fn `Respawn`)

(fn `UserConstructionScript`)