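; Crater hazard actor that destroys the TopDownCharacter when it touches the Cone component.
; Both hit and begin-overlap events on the Cone cast the other actor, destroy it and print a debug message.
; An unused TeleportPlayerToStart function checks the player pawn's class, then only resets headset position tracking via ResetOrientationAndPosition, without moving the character.
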(event `self.Cone.OnComponentHit`
  (params (HitComponent :type "PrimitiveComponent Object Reference") (OtherActor :type "Actor Object Reference") (OtherComp :type "PrimitiveComponent Object Reference") (NormalImpulse :type "Vector Structure") (Hit :type "HitResult Structure (by ref)"))
  (bind _astop_down_character (cast `/Game/Blueprints/TopDownCharacter` OtherActor))
  (`self.K2_DestroyActor` _astop_down_character)
  (`KismetSystemLibrary.PrintString` "You touched a crater"))

(event `self.Cone.OnComponentBeginOverlap`
  (params (OverlappedComponent :type "PrimitiveComponent Object Reference") (OtherActor :type "Actor Object Reference") (OtherComp :type "PrimitiveComponent Object Reference") (OtherBodyIndex :type Integer) (bFromSweep :type Boolean) (SweepResult :type "HitResult Structure (by ref)"))
  (bind _astop_down_character (cast `/Game/Blueprints/TopDownCharacter` OtherActor))
  (`self.K2_DestroyActor` _astop_down_character)
  (`KismetSystemLibrary.PrintString` "You touched a crater"))

(fn `TeleportPlayerToStart`
  (cast `/Game/Blueprints/TopDownCharacter` (`GameplayStatics.GetPlayerPawn` 0))
  (`HeadMountedDisplayFunctionLibrary.ResetOrientationAndPosition` 0.0 "Position"))

(fn `UserConstructionScript`)