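; Star_3 is an actor, apparently the third level-progression star, that hides itself on BeginPlay and can unlock the next level.
; OpenLevel and OpenLevel3 check that player 0's pawn is a TopDownCharacter, destroy their respective wall, print an unlock message and destroy the star.
; OpenLevel3 also sets EndGame after the destroy call.
; Nothing in this Blueprint calls either function, reveals the star or acts on EndGame.
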(event `self.ReceiveBeginPlay`
  (`self.SetActorHiddenInGame` true))

(fn `OpenLevel`
  (cast `/Game/Blueprints/TopDownCharacter` (`GameplayStatics.GetPlayerPawn` 0))
  (`self.K2_DestroyActor` (`self.WallToDestroy`))
  (`KismetSystemLibrary.PrintString` "Next level unlocked!")
  (`self.K2_DestroyActor`))

(fn `OpenLevel3`
  (cast `/Game/Blueprints/TopDownCharacter` (`GameplayStatics.GetPlayerPawn` 0))
  (`self.K2_DestroyActor` (`self.WallToDestroy3`))
  (`KismetSystemLibrary.PrintString` "Next level unlocked!")
  (`self.K2_DestroyActor`)
  (set `self.EndGame` true))

(fn `UserConstructionScript`)